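; Floor actor that the player tilts with input, which is enabled once something overlaps its trigger volume.
; MoveX scales by Initvalue to set absolute roll and pitch on the floor, spin cube and Walls 2–4, and shifts Walls 1 and 2 from hard-coded offsets.
; G resets only the main floor to OrignPoint; MoveY is unused.
; Wall2's location prints on screen as debug output.
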(event OnComponentBeginOverlap(triggerVolume)
  (params (OtherActor :type Actor%20Object%20Reference) (OtherComp :type Primitive%20Component%20Object%20Reference) (OtherBodyIndex :type Integer) (bFromSweep :type Boolean) (SweepResult :type Hit%20Result%20Structure%20%28by%20ref%29))
  (Input|EnableInput (Game|GetPlayerController 0)))

(event Input|AxisEvents|InputAxisMoveX
  (params (AxisValue :type Float%20%28single-precision%29))
  (bind _initvalue (Variables|Default|Getinitvalue))
  (bind _wall2 (Variables|boxs|GetWall2))
  (bind _returnvalue (* AxisValue _initvalue -1e+01))
  (bind _relativelocation (Variables|/Script/Engine.SceneComponent|GetRelativeLocation _wall2))
  (bind (_x _y _z) (Math|Vector|BreakVector _relativelocation))
  ;[1 1 1] Control the floor
  (Transformation|SetRelativeRotation (Variables|Default|GetMainFloors) (Math|Rotator|MakeRotator _returnvalue (* (stale Input|AxisEvents|InputAxisMoveY AxisValue) (Variables|Default|Getinitvalue) -1e+01) 0.0) false false)
  (Transformation|SetRelativeRotation (Variables|boxs|GetWall3) (Math|Rotator|MakeRotator (* (stale Input|AxisEvents|InputAxisMoveY AxisValue) (Variables|Default|Getinitvalue) -1e+01) _returnvalue 9e+01) false false)
  (Transformation|SetRelativeLocationAndRotation _wall2 (Math|Vector|MakeVector (+ _returnvalue 0.0) (+ (* (stale Input|AxisEvents|InputAxisMoveY AxisValue) (Variables|Default|Getinitvalue) -1e+01) -4.4e+02) 9e+01) (Math|Rotator|MakeRotator _returnvalue (* (stale Input|AxisEvents|InputAxisMoveY AxisValue) (Variables|Default|Getinitvalue) -1e+01) 0.0) false false)
  (Transformation|SetRelativeLocation (Variables|boxs|GetWall1) (Math|Vector|MakeVector (+ _returnvalue 0.0) (+ (* (stale Input|AxisEvents|InputAxisMoveY AxisValue) (Variables|Default|Getinitvalue) -1e+01) 4.6e+02) 9e+01) false false)
  (Development|PrintString (Utilities|String|ToString(Vector) (Math|Vector|MakeVector _x _y _z)) (Variables|Default|GetTrue)))

(event Input|AxisEvents|InputAxisMoveY
  (params (AxisValue :type Float%20%28single-precision%29))
  ;[1 1 1] Control the floor
)

(event Input|KeyboardEvents|G
  (params (Key :type Key%20Structure :default "AnyKey"))
  ;[1 1 1] Set Floor to Orign
  (:Pressed
    (Transformation|SetRelativeRotation (Variables|Default|GetMainFloors) (Variables|Default|GetOrignPoint) false false)))

(fn ConstructionScript)